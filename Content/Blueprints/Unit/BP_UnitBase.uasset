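; BP_UnitBase is a unit base Blueprint that handles movement requests and shows the unit's selection state.
; Move, rotate and snap events pass straight through to the ACSimpleMovement component.
; The Selected event adds a circle plane with a dynamic material on first click, tinting it cyan for Clicked and destroying it for None.
; Snapped only recolors the existing circle red, without creating one.
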(event `/Game/Blueprints/Unit/Interface/BPI_Control.MoveToTarget`
  (params (TargetLocation :type "Vector Structure") (TargetActor :type "Actor Object Reference"))
  (`/Game/Blueprints/Unit/AC_SimpleMovement.MoveToTarget` (`self.AC_SimpleMovement`) TargetLocation TargetActor))

(event `/Game/Blueprints/Unit/Interface/BPI_Control.RotateToTarget`
  (params (TargetLocation :type "Vector Structure") (TargetActor :type "Actor Object Reference"))
  (`/Game/Blueprints/Unit/AC_SimpleMovement.RotateToTarget` (`self.AC_SimpleMovement`) TargetLocation TargetActor))

(event `/Game/Blueprints/Unit/Interface/BPI_Control.SnapToTarget`
  (params (TargetActor :type "Actor Object Reference"))
  (`/Game/Blueprints/Unit/AC_SimpleMovement.SnapToTarget` (`self.AC_SimpleMovement`) TargetActor))

(event `/Game/Blueprints/Unit/Interface/BPI_Control.Selected`
  (params (SelectedState :type "/Game/Blueprints/Unit/Enum/E_SelectedState Enum" :default "NewEnumerator0"))
  (switch `/Game/Blueprints/Unit/Enum/E_SelectedState` SelectedState
    (:`NewEnumerator0`
      (`ActorComponent.K2_DestroyComponent` (`self.Plane`)))
    (:`NewEnumerator1`
      (`/Engine/EditorBlueprintResources/StandardMacros.IsValid` (`self.Plane`)
        (:`Is Valid`
          (`MaterialInstanceDynamic.SetVectorParameterValue` (`self.CircleMaterial`) "Color" (struct :`R` 0.122139 :`G` 0.938686 :`B` 0.991102 :`A` 1.0)))
        (:`Is Not Valid`
          (bind _returnvalue (`AddComponent|NODE_AddStaticMeshComponent-0` :`RelativeTransform` (`KismetMathLibrary.MakeTransform` (0.0 0.0 -50.0) (struct) (2.0 2.0 2.0))))
          (bind _output_get (set `self.Plane` _returnvalue))
          (bind _returnvalue_2 (`PrimitiveComponent.CreateDynamicMaterialInstance` _output_get 0 "/Game/Assets/Material/MI_SelectionCircle.MI_SelectionCircle" "None"))
          (bind _output_get_2 (set `self.CircleMaterial` _returnvalue_2))
          (`MaterialInstanceDynamic.SetVectorParameterValue` _output_get_2 "Color" (struct :`R` 0.122139 :`G` 0.938686 :`B` 0.991102 :`A` 1.0)))))
    (:`NewEnumerator2`
      (`MaterialInstanceDynamic.SetVectorParameterValue` (`self.CircleMaterial`) "Color" (struct :`R` 0.666667 :`G` 0.012241 :`A` 1.0)))))

(fn `UserConstructionScript`)
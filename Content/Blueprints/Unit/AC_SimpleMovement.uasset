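; Unit movement component that moves and yaw-rotates its owning actor toward targets at constant speed.
; MoveToTarget, RotateToTarget and SnapToTarget set targets and flags; Tick then interpolates, landing exactly on the final step, with swept moves.
; An actor move target is sampled only once, while SnapToTarget continuously faces a moving actor until cleared.
; Unsnapped rotation uses only the stored location, so an actor passed to RotateToTarget does not set the aim.
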(event `self.ReceiveBeginPlay`
  (set `self.Owner` (`self.GetOwner`)))

(event `self.ReceiveTick`
  (params (DeltaSeconds :type "Float (single-precision)"))
  (`|ExecutionSequence`
    (:`then_0`
      (if (`self.IsMoving`)
        (`self.MovingToTarget` DeltaSeconds)))
    (:`then_1`
      (if (`self.IsRotating`)
        (`self.RotatingToTarget` DeltaSeconds)))))

(fn `MoveToTarget`
  (params (TargetLocation :type "Vector Structure") (TargetActor :type "Actor Object Reference"))
  (`/Engine/EditorBlueprintResources/StandardMacros.IsValid` TargetActor
    (:`Is Valid`
      (bind _output_get (set `self.TargetActorToMove` TargetActor))
      (set `self.TargetLocationToMove` (`Actor.K2_GetActorLocation` _output_get)))
    (:`Is Not Valid`
      (set `self.TargetLocationToMove` TargetLocation)))
  (set `self.IsMoving` true))

(fn `MovingToTarget`
  (params (DeltaSeconds :type "Float (double-precision)"))
  (locals (CurrentLocation :type "Vector Structure" :default (0.0 0.0 0.0)))
  (bind _returnvalue (> (* (`self.CurrentSpeed`) (`local.DeltaSeconds`)) (`KismetMathLibrary.Vector_Distance` (`local.CurrentLocation`) (`self.TargetLocationToMove`))))
  (set `local.CurrentLocation` (`Actor.K2_GetActorLocation` (`self.Owner`)))
  (`Actor.K2_SetActorLocation` (`self.Owner`) (`KismetMathLibrary.SelectVector` (`self.TargetLocationToMove`) (`KismetMathLibrary.VInterpTo_Constant` (`local.CurrentLocation`) (`self.TargetLocationToMove`) (`local.DeltaSeconds`) (`self.CurrentSpeed`)) _returnvalue) true false)
  (if _returnvalue
    (set `self.IsMoving` false)))

(fn `RotateToTarget`
  (params (TargetLocation :type "Vector Structure") (TargetActor :type "Actor Object Reference"))
  (`/Engine/EditorBlueprintResources/StandardMacros.IsValid` TargetActor
    (:`Is Valid`
      (set `self.TargetActorToRotate` TargetActor))
    (:`Is Not Valid`
      (set `self.TargetLocationToRotate` TargetLocation)))
  (set `self.IsRotating` true))

(fn `RotatingToTarget`
  (params (DeltaSeconds :type "Float (double-precision)"))
  (locals (TargetActorLocationToRotate :type "Vector Structure") (CurrentRotation :type "Rotator Structure" :default (struct)) (TargetRotation :type "Rotator Structure" :default (struct)))
  (bind _owner (`self.Owner`))
  (bind (_returnvalue_roll _returnvalue_pitch _returnvalue_yaw) (`KismetMathLibrary.BreakRotator` (`KismetMathLibrary.NormalizedDeltaRotator` (`local.CurrentRotation`) (`local.TargetRotation`))))
  (bind (_returnvalue_roll_2 _returnvalue_pitch_2 _returnvalue_yaw_2) (`KismetMathLibrary.BreakRotator` (`Actor.K2_GetActorRotation` _owner)))
  (bind (_returnvalue_roll_3 _returnvalue_pitch_3 _returnvalue_yaw_3) (`KismetMathLibrary.BreakRotator` (`KismetMathLibrary.FindLookAtRotation` (`Actor.K2_GetActorLocation` _owner) (`KismetMathLibrary.SelectVector` (`local.TargetActorLocationToRotate`) (`self.TargetLocationToRotate`) (`self.IsSnapped`)))))
  (bind _returnvalue (> (* (`self.CurrentRotateSpeed`) (`local.DeltaSeconds`)) (`KismetMathLibrary.Abs` _returnvalue_yaw)))
  (`/Engine/EditorBlueprintResources/StandardMacros.IsValid` (`self.TargetActorToRotate`)
    (:`Is Valid`
      (set `local.TargetActorLocationToRotate` (`Actor.K2_GetActorLocation` (`self.TargetActorToRotate`))))
    (:`Is Not Valid`
      _))
  (set `local.CurrentRotation` (`KismetMathLibrary.MakeRotator` 0.0 0.0 _returnvalue_yaw_2))
  (set `local.TargetRotation` (`KismetMathLibrary.MakeRotator` 0.0 0.0 _returnvalue_yaw_3))
  (`Actor.K2_SetActorRotation` (`self.Owner`) (`KismetMathLibrary.SelectRotator` (`local.TargetRotation`) (`KismetMathLibrary.RInterpTo_Constant` (`local.CurrentRotation`) (`local.TargetRotation`) (`local.DeltaSeconds`) (`self.CurrentRotateSpeed`)) _returnvalue) false)
  (if (and _returnvalue (not (`self.IsSnapped`)))
    (set `self.IsRotating` false)))

(fn `SnapToTarget`
  (params (TargetActor :type "Actor Object Reference"))
  (`/Engine/EditorBlueprintResources/StandardMacros.IsValid` TargetActor
    (:`Is Valid`
      (set `self.TargetActorToRotate` TargetActor)
      (set `self.IsRotating` true)
      (set `self.IsSnapped` true))
    (:`Is Not Valid`
      (set `self.TargetActorToRotate` null)
      (set `self.IsRotating` false)
      (set `self.IsSnapped` false))))
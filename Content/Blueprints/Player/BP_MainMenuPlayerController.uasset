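; Player controller for the main menu that creates the W_MainMenu widget on BeginPlay, adds it to the viewport and switches to UI-only input without mouse lock.
; It also works with stats and inventory-equipment components, passing equipment stat changes into the stats component as non-base stats.
; A getter exposes the inventory-equipment component, while the stats component's own change event is left empty.
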(event `self.ReceiveBeginPlay`
  (bind _returnvalue (`|CreateWidget` "/Game/Blueprints/GameMode/Widget/W_MainMenu.W_MainMenu_C" self))
  (bind _output_get (set `self.W_MainMenu` _returnvalue))
  (`UserWidget.AddToViewport` _output_get 0)
  (`WidgetBlueprintLibrary.SetInputMode_UIOnlyEx` self (`self.W_MainMenu`)))

(event `self.AC_Stats.StatsChanged`
  (params (Stats :type "Map of /Game/Blueprints/InventoryEquipment/Enum/E_StatCategory Enum to /Game/Blueprints/InventoryEquipment/Struct/S_StatAmounts Structure" :default _)))

(event `self.AC_InventoryEquipment.StatsChanged`
  (params (Stats :type "Map of /Game/Blueprints/InventoryEquipment/Enum/E_StatCategory Enum to /Game/Blueprints/InventoryEquipment/Struct/S_StatAmounts Structure" :default _))
  (`/Game/Blueprints/Stat/AC_Stats.AddStat` (`self.AC_Stats`) "NewEnumerator0" false Stats))

(fn `GetInventoryEquipment`
  (returns (InventoryEquipment :type "/Game/Blueprints/InventoryEquipment/AC_InventoryEquipment Object Reference"))
  (return (`self.AC_InventoryEquipment`)))

(fn `UserConstructionScript`
  (`parent.UserConstructionScript`))
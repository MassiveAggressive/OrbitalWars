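; Actor component that stores stats per source in base and additive maps and maintains their combined totals.
; AddStat writes a source's stats into the chosen map, then nested enum loops sum amounts by category and addition type across all sources.
; It merges both sums into AddedStats, clears the scratch maps and calls StatsChanged with the result.
; Unconnected leftovers include older summing logic and a debug print.
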(fn `AddStat`
  (params (StatsFrom :type "/Game/Blueprints/Stat/StatsEnum/E_StatsFrom Enum" :default "NewEnumerator1") (ToBase :type Boolean) (Stats :type "Map of /Game/Blueprints/InventoryEquipment/Enum/E_StatCategory Enum to /Game/Blueprints/InventoryEquipment/Struct/S_StatAmounts Structure"))
  (locals (BaseAmountsRef :type "Map of /Game/Blueprints/InventoryEquipment/Enum/E_StatAdditionType Enum to Float (double-precision)") (AdditiveAmountsRef :type "Map of /Game/Blueprints/InventoryEquipment/Enum/E_StatAdditionType Enum to Float (double-precision)") (AddedAmountsRef :type "Map of /Game/Blueprints/InventoryEquipment/Enum/E_StatAdditionType Enum to Float (double-precision)") (StatsFromRef :type "/Game/Blueprints/Stat/StatsEnum/E_StatsFrom Enum") (StatCategoryRef :type "/Game/Blueprints/InventoryEquipment/Enum/E_StatCategory Enum") (StatAditionType :type "/Game/Blueprints/InventoryEquipment/Enum/E_StatAdditionType Enum") (S_StatsRef :type "Map of /Game/Blueprints/InventoryEquipment/Enum/E_StatCategory Enum to /Game/Blueprints/InventoryEquipment/Struct/S_StatAmounts Structure"))
  (bind _statcategoryref (`local.StatCategoryRef`))
  (bind _statcategoryref_2 (`local.StatCategoryRef`))
  (bind _amounts (break `/Game/Blueprints/InventoryEquipment/Struct/S_StatAmounts` (`BlueprintMapLibrary.Map_Find` (`self.AddedBaseStats`) _statcategoryref)))
  (bind _amounts_2 (break `/Game/Blueprints/InventoryEquipment/Struct/S_StatAmounts` (`BlueprintMapLibrary.Map_Find` (`self.AddedAdditiveStats`) _statcategoryref)))
  (`BlueprintMapLibrary.Map_Add` (select `bool` ToBase :`false` (`self.AdditiveStats`) :`true` (`self.BaseStats`)) StatsFrom (make `/Game/Blueprints/Stat/StatsStruct/S_Stats` Stats))
  (bind _enumvalue (foreach `/Game/Blueprints/Stat/StatsEnum/E_StatsFrom` false)
    (:`LoopBody`
      (set `local.StatsFromRef` _enumvalue)
      (bind _enumvalue_2 (foreach `/Game/Blueprints/InventoryEquipment/Enum/E_StatCategory` false)
        (:`LoopBody`
          (set `local.StatCategoryRef` _enumvalue_2)
          (bind _enumvalue_3 (foreach `/Game/Blueprints/InventoryEquipment/Enum/E_StatAdditionType` false)
            (:`LoopBody`
              (bind _output_get (set `local.StatAditionType` _enumvalue_3))
              (`BlueprintMapLibrary.Map_Add` (`local.BaseAmountsRef`) _output_get (+ (`BlueprintMapLibrary.Map_Find` (`.Amounts_26_0915A13F4F6A65445893A8A768B38F02` (break `/Game/Blueprints/InventoryEquipment/Struct/S_StatAmounts` (`BlueprintMapLibrary.Map_Find` (`self.AddedBaseStats`) (`local.StatCategoryRef`)))) _output_get) (`BlueprintMapLibrary.Map_Find` (`.Amounts_26_0915A13F4F6A65445893A8A768B38F02` (break `/Game/Blueprints/InventoryEquipment/Struct/S_StatAmounts` (`BlueprintMapLibrary.Map_Find` (`.Stats_11_11419B8A445CB92626D55E9B59AC1FFF` (break `/Game/Blueprints/Stat/StatsStruct/S_Stats` (`BlueprintMapLibrary.Map_Find` (`self.BaseStats`) (`local.StatsFromRef`)))) (`local.StatCategoryRef`)))) (`local.StatAditionType`))))
              (`BlueprintMapLibrary.Map_Add` (`local.AdditiveAmountsRef`) (`local.StatAditionType`) (+ (`BlueprintMapLibrary.Map_Find` (`.Amounts_26_0915A13F4F6A65445893A8A768B38F02` (break `/Game/Blueprints/InventoryEquipment/Struct/S_StatAmounts` (`BlueprintMapLibrary.Map_Find` (`self.AddedAdditiveStats`) (`local.StatCategoryRef`)))) (`local.StatAditionType`)) (`BlueprintMapLibrary.Map_Find` (`.Amounts_26_0915A13F4F6A65445893A8A768B38F02` (break `/Game/Blueprints/InventoryEquipment/Struct/S_StatAmounts` (`BlueprintMapLibrary.Map_Find` (`.Stats_11_11419B8A445CB92626D55E9B59AC1FFF` (break `/Game/Blueprints/Stat/StatsStruct/S_Stats` (`BlueprintMapLibrary.Map_Find` (`self.AdditiveStats`) (`local.StatsFromRef`)))) (`local.StatCategoryRef`)))) (`local.StatAditionType`)))))
            (:`then`
              (`BlueprintMapLibrary.Map_Add` (`self.AddedBaseStats`) (`local.StatCategoryRef`) (make `/Game/Blueprints/InventoryEquipment/Struct/S_StatAmounts` (`local.BaseAmountsRef`)))
              (`BlueprintMapLibrary.Map_Add` (`self.AddedAdditiveStats`) (`local.StatCategoryRef`) (make `/Game/Blueprints/InventoryEquipment/Struct/S_StatAmounts` (`local.AdditiveAmountsRef`))))))))
    (:`then`
      (bind _enumvalue_4 (foreach `/Game/Blueprints/InventoryEquipment/Enum/E_StatCategory` false)
        (:`LoopBody`
          (set `local.StatCategoryRef` _enumvalue_4)
          (`BlueprintMapLibrary.Map_Add` (`self.AddedStats`) (`local.StatCategoryRef`) (make `/Game/Blueprints/InventoryEquipment/Struct/S_StatAmounts` (`|MakeMap` "NewEnumerator0" (+ (`BlueprintMapLibrary.Map_Find` _amounts "NewEnumerator0") (`BlueprintMapLibrary.Map_Find` _amounts_2 "NewEnumerator0")) "NewEnumerator1" (+ (`BlueprintMapLibrary.Map_Find` _amounts "NewEnumerator1") (`BlueprintMapLibrary.Map_Find` _amounts_2 "NewEnumerator1")) :!type "/Game/Blueprints/InventoryEquipment/Enum/E_StatAdditionType Enum")))
          (`BlueprintMapLibrary.Map_Add` (`self.AddedBaseStats`) _statcategoryref_2 (make `/Game/Blueprints/InventoryEquipment/Struct/S_StatAmounts` _))
          (`BlueprintMapLibrary.Map_Add` (`self.AddedAdditiveStats`) _statcategoryref_2 (make `/Game/Blueprints/InventoryEquipment/Struct/S_StatAmounts` _)))
        (:`then`
          (`self.StatsChanged` (`self.AddedStats`)))))))